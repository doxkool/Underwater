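; BP_Gate is a gate actor that opens and closes, tied to the game's lobby state.
; On BeginPlay the authority binds EA_CloseGates to the kernel game state's lobby-state event; EA_OpenGate is not bound here.
; Both EA events forward to MC events: opening offsets the Gate component upward instantly, and closing restores its stored default relative location.
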(event Custom|EA_OpenGate
  (CallFunction|MCOpenGate))

(event Custom|EA_CloseGates
  (CallFunction|MCCloseGate))

(event Custom|MC_OpenGate
  (Transformation|AddLocalOffset (Variables|Default|GetGate) "0.000000, 0,500.000000" false false))

(event Custom|MC_CloseGate
  (Transformation|SetRelativeLocation (Variables|Default|GetGate) (Variables|Default|GetDefaultLocation) false false))

(event EventBeginPlay
  (Networking|SwitchHasAuthority
    (:Authority
      (EventDispatchers|BindEventtoDLobbyState (CallFunction|HKernelGS) (delegate Custom|EA_CloseGates)))))

(fn ConstructionScript)