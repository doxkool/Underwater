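; BP_Generator is a networked generator actor that can be repaired and shows its state by colour.
; On BeginPlay the server binds its reset event to the Kernel game state's lobby-state delegate, which clears IsRepaired.
; A separate repair event sets IsRepaired, and its RepNotify swaps six cube meshes between green and red tile materials.
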(event Custom|EA_Repair
  (Variables|Default|SetIsRepaired true))

(event Custom|EA_Reset
  (Variables|Default|SetIsRepaired false))

(event EventBeginPlay
  (Networking|SwitchHasAuthority
    (:Authority
      (EventDispatchers|BindEventtoDLobbyState (CallFunction|HKernelGS) (delegate Custom|EA_Reset)))))

(fn ConstructionScript)

(fn OnRepIsRepaired
  (bind _cube2 (Variables|Default|GetCube2))
  (if (Variables|Default|GetIsRepaired)
    (Rendering|Material|SetMaterial _cube2 0 "/Game/Materials/MI_Green.MI_Green")
    (else
      (Rendering|Material|SetMaterial _cube2 0 "/Game/Materials/MI_TilesRed.MI_TilesRed"))))