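; HUD Blueprint that manages the owning player's widgets across lobby, round and finish phases, plus chat, kill feed and notifications.
; BeginPlay shows a widget matching the current GameState phase (observer HUD if play is underway), then binds to GameState dispatchers.
; Phase events clear main widgets via FRemoveAll before switching, while message events feed chat, kill feed and notifications.
; Toggle functions lazily create and cache widgets, layering overlays by Z-order.
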(event Custom|E_OnGameStartDelay
  ;[1 1 1] Show loading screen
  (WidgetRemoving|FRemoveAll)
  (MainWidgets|FToggleLoadingScreen true))

(event Custom|E_Notify
  (params (Message :type String))
  ;[1 1 1] Notification
  (Notify|FShowNotify Message))

(event Custom|E_OnRoundStart
  (bind _playerowner (Variables|Default|GetPlayerOwner))
  ;[1 1 1] Round start - show wait screen for hunters
  (WidgetRemoving|FRemoveAll)
  (Variables|/Script/Engine.PlayerController|SetbShowMouseCursor _playerowner false)
  (Input|SetInputModeGameOnly _playerowner))

(event Custom|E_OnRoundFinish
  ;[1 1 1] Round Finish - show round finish widget with winner name
  (WidgetRemoving|FRemoveAll)
  (MainWidgets|FToggleRoundFinishScreen true))

(event Custom|E_OnPlayTime
  ;[1 1 1] Play time start - Show player hud and kill feed
  (WidgetRemoving|FRemoveAll)
  (MainWidgets|FTogglePlayerHud true)
  (MainWidgets|FToggleKillFeed true))

(event Custom|E_UpdateLobbyChat
  (params (PlayerId :type Integer) (Message :type String))
  ;[1 1 1] Update lobby chat
  (Default|EAddLobbyMessage (Variables|WidgetsRefs|GetLobby) PlayerId Message))

(event Custom|E_UpdateKillFeed
  (params (KillerId :type Integer) (VictimId :type Integer))
  (bind _killfeed (Variables|WidgetsRefs|GetKillFeed))
  ;[1 1 1] Update kill feed
  (bind _returnvalue (UserInterface|CreateWidget "/Game/Blueprints/Widgets/Game/BP_WE_KillFeedMessage.BP_WE_KillFeedMessage_C" (Variables|Default|GetPlayerOwner) KillerId VictimId))
  (Utilities|IsValid _killfeed
    (:Is%20Valid
      (Default|EAddMessage _killfeed _returnvalue))
    (:Is%20Not%20Valid
      (MainWidgets|FToggleKillFeed true)
      (Default|EAddMessage (Variables|WidgetsRefs|GetKillFeed) _returnvalue))))

(event Custom|E_ShowLobby
  ;[1 1 1] Lobby state
  (WidgetRemoving|FRemoveAll)
  (MainWidgets|FToggleLobby true))

(event Custom|E_UpdateGameChat
  (params (IsServer :type Boolean) (SenderId :type Integer) (Message :type String))
  ;[1 1 1] Update game chat
  (UserCalledWidgets|FToggleGameChat true)
  (Default|EAddMessage (Variables|WidgetsRefs|GetGameChat) IsServer SenderId Message))

(event EventBeginPlay
  (Utilities|IsValid (Game|GetGameState)
    (:Is%20Valid
      _)
    (:Is%20Not%20Valid
      (Utilities|FlowControl|Delay 1.0)))
  (Utilities|FlowControl|Sequence
    (:then_0
      ;[1 1 1] Define what widget to show on begin play
      (Utilities|FlowControl|Sequence
        (:then_0
          (WidgetRemoving|FRemoveAll))
        (:then_1
          (switch Utilities|FlowControl|Switch|SwitchonE_GlobalState (Variables|/Game/Blueprints/Kernel/BP_Kernel_GS.BP_Kernel_GS_C|GetGlobalState (CallFunction|HKernelGS))
            (:NewEnumerator29
              (MainWidgets|FToggleLobby true))
            (:NewEnumerator17
              (MainWidgets|FToggleOserverHud true))
            (:NewEnumerator27
              (MainWidgets|FToggleRoundFinishScreen true))))))
    (:then_1
      ;[1 1 1] Show loading screen
      (EventDispatchers|BindEventtoDGameStartDelay (CallFunction|HKernelGS) (delegate Custom|E_OnGameStartDelay)))
    (:then_2
      ;[1 1 1] Lobby state
      (EventDispatchers|BindEventtoDLobbyState (CallFunction|HKernelGS) (delegate Custom|E_ShowLobby)))
    (:then_3
      ;[1 1 1] Round start - show wait screen for hunters
      (EventDispatchers|BindEventtoDRoundStart (CallFunction|HKernelGS) (delegate Custom|E_OnRoundStart)))
    (:then_4
      ;[1 1 1] Play time start - Show player hud and kill feed
      (EventDispatchers|BindEventtoDPlayTime (CallFunction|HKernelGS) (delegate Custom|E_OnPlayTime)))
    (:then_5
      ;[1 1 1] Round Finish - show round finish widget with winner name
      (EventDispatchers|BindEventtoDRoundFinish (CallFunction|HKernelGS) (delegate Custom|E_OnRoundFinish)))
    (:then_6
      ;[1 1 1] Update kill feed
      (EventDispatchers|BindEventtoDUpdateKillFeed (CallFunction|HKernelGS) (delegate Custom|E_UpdateKillFeed)))
    (:then_7
      ;[1 1 1] Update game chat
      (EventDispatchers|BindEventtoDUpdateGameChat (CallFunction|HKernelGS) (delegate Custom|E_UpdateGameChat))
      ;[1 1 1] Update lobby chat
      (EventDispatchers|BindEventtoDUpdateLobbyChat (CallFunction|HKernelGS) (delegate Custom|E_UpdateLobbyChat))
      ;[1 1 1] Notification
      (EventDispatchers|BindEventtoDNotify (CallFunction|HKernelGS) (delegate Custom|E_Notify)))))

(fn ConstructionScript)

(fn FTogglePlayerHud
  (params (Show :type Boolean))
  (if Show
    (Variables|WidgetsRefs|GetPlayerHud
      (:then
        (Utilities|MHIsWidgetVisible (Variables|WidgetsRefs|GetPlayerHud)
          (:false
            (UserInterface|Viewport|AddtoViewport (Variables|WidgetsRefs|GetPlayerHud) 0))))
      (:else
        (bind _returnvalue (UserInterface|CreateWidget "/Game/Blueprints/Widgets/Game/BP_W_HUD.BP_W_HUD_C" (Variables|Default|GetPlayerOwner)))
        (bind _output_get (Variables|WidgetsRefs|SetPlayerHud _returnvalue))
        (UserInterface|Viewport|AddtoViewport _output_get 0)))
    (else
      (bind _playerhud (Variables|WidgetsRefs|GetPlayerHud)
        (:then
          (Widget|RemovefromParent _playerhud))
        (:else)))))

(fn FToggleLobby
  (params (Show :type Boolean))
  (if Show
    (Variables|WidgetsRefs|GetLobby
      (:then
        (Utilities|MHIsWidgetVisible (Variables|WidgetsRefs|GetLobby)
          (:false
            (UserInterface|Viewport|AddtoViewport (Variables|WidgetsRefs|GetLobby) 0))))
      (:else
        (bind _returnvalue (UserInterface|CreateWidget "/Game/Blueprints/Widgets/Lobby/BP_W_Lobby.BP_W_Lobby_C" (Variables|Default|GetPlayerOwner)))
        (bind _output_get (Variables|WidgetsRefs|SetLobby _returnvalue))
        (UserInterface|Viewport|AddtoViewport _output_get 0)))
    (else
      (bind _lobby (Variables|WidgetsRefs|GetLobby)
        (:then
          (Widget|RemovefromParent _lobby))
        (:else)))))

(fn FToggleOserverHud
  (params (Show :type Boolean))
  (if Show
    (Variables|WidgetsRefs|GetObserverHudWB
      (:then
        (Utilities|MHIsWidgetVisible (Variables|WidgetsRefs|GetObserverHudWB)
          (:false
            (UserInterface|Viewport|AddtoViewport (Variables|WidgetsRefs|GetObserverHudWB) 0))))
      (:else
        (bind _returnvalue (UserInterface|CreateWidget "/Game/Blueprints/Widgets/Game/BP_W_ObserverHud.BP_W_ObserverHud_C" (Variables|Default|GetPlayerOwner)))
        (bind _output_get (Variables|WidgetsRefs|SetObserverHudWB _returnvalue))
        (UserInterface|Viewport|AddtoViewport _output_get 0)))
    (else
      (bind _observerhudwb (Variables|WidgetsRefs|GetObserverHudWB)
        (:then
          (Widget|RemovefromParent _observerhudwb)
          (return))
        (:else)))))

(fn FToggleKillFeed
  (params (Show :type Boolean))
  (if Show
    (Variables|WidgetsRefs|GetKillFeed
      (:then
        (Utilities|MHIsWidgetVisible (Variables|WidgetsRefs|GetKillFeed)
          (:false
            (UserInterface|Viewport|AddtoViewport (Variables|WidgetsRefs|GetKillFeed) 0))))
      (:else
        (bind _returnvalue (UserInterface|CreateWidget "/Game/Blueprints/Widgets/Game/BP_W_KillFeed.BP_W_KillFeed_C" (Variables|Default|GetPlayerOwner)))
        (bind _output_get (Variables|WidgetsRefs|SetKillFeed _returnvalue))
        (UserInterface|Viewport|AddtoViewport _output_get 0)))
    (else
      (bind _killfeed (Variables|WidgetsRefs|GetKillFeed)
        (:then
          (Widget|RemovefromParent _killfeed))
        (:else)))))

(fn FToggleinGameMenu
  (params (Show :type Boolean))
  (if Show
    (Variables|WidgetsRefs|GetInGameMenu
      (:then
        (Utilities|MHIsWidgetVisible (Variables|WidgetsRefs|GetInGameMenu)
          (:false
            (UserInterface|Viewport|AddtoViewport (Variables|WidgetsRefs|GetInGameMenu) 99))))
      (:else
        (bind _returnvalue (UserInterface|CreateWidget "/Game/Blueprints/Widgets/Game/BP_W_InGameMenu.BP_W_InGameMenu_C" (Variables|Default|GetPlayerOwner)))
        (bind _output_get (Variables|WidgetsRefs|SetInGameMenu _returnvalue))
        (UserInterface|Viewport|AddtoViewport _output_get 99)))
    (else
      (bind _ingamemenu (Variables|WidgetsRefs|GetInGameMenu)
        (:then
          (Widget|RemovefromParent _ingamemenu))
        (:else)))))

(fn FRemoveAll
  (Utilities|FlowControl|Sequence
    (:then_0
      (bind _playerhud (Variables|WidgetsRefs|GetPlayerHud)
        (:then
          (Widget|RemovefromParent _playerhud)
          (Variables|WidgetsRefs|SetPlayerHud 0))
        (:else)))
    (:then_1
      (bind _observerhudwb (Variables|WidgetsRefs|GetObserverHudWB)
        (:then
          (Widget|RemovefromParent _observerhudwb)
          (Variables|WidgetsRefs|SetObserverHudWB 0))
        (:else)))
    (:then_2
      (bind _killfeed (Variables|WidgetsRefs|GetKillFeed)
        (:then
          (Widget|RemovefromParent _killfeed)
          (Variables|WidgetsRefs|SetKillFeed 0))
        (:else)))
    (:then_3
      (bind _lobby (Variables|WidgetsRefs|GetLobby)
        (:then
          (Widget|RemovefromParent _lobby)
          (Variables|WidgetsRefs|SetLobby 0))
        (:else)))
    (:then_4
      (bind _killfeed_2 (Variables|WidgetsRefs|GetKillFeed)
        (:then
          (Widget|RemovefromParent _killfeed_2)
          (Variables|WidgetsRefs|SetKillFeed 0))
        (:else)))
    (:then_5
      (bind _roundfinishscreen (Variables|WidgetsRefs|GetRoundFinishScreen)
        (:then
          (Widget|RemovefromParent _roundfinishscreen)
          (Variables|WidgetsRefs|SetRoundFinishScreen 0))
        (:else)))
    (:then_6
      (bind _gamechat (Variables|WidgetsRefs|GetGameChat)
        (:then
          (Widget|RemovefromParent _gamechat)
          (Variables|WidgetsRefs|SetGameChat 0))
        (:else)))))

(fn FToggleLoadingScreen
  (params (Show :type Boolean))
  (if Show
    (Variables|WidgetsRefs|GetLoadingScreen
      (:then
        (Utilities|MHIsWidgetVisible (Variables|WidgetsRefs|GetLoadingScreen)
          (:false
            (UserInterface|Viewport|AddtoViewport (Variables|WidgetsRefs|GetLoadingScreen) 0))))
      (:else
        (bind _returnvalue (UserInterface|CreateWidget "/Game/Blueprints/Widgets/Game/BP_W_LoadingScreen.BP_W_LoadingScreen_C" (Variables|Default|GetPlayerOwner) (Math|Conversions|ToFloat(Integer) (Variables|/Game/Blueprints/Kernel/BP_Kernel_GS.BP_Kernel_GS_C|GetGameStartDelayS (CallFunction|HKernelGS)))))
        (bind _output_get (Variables|WidgetsRefs|SetLoadingScreen _returnvalue))
        (UserInterface|Viewport|AddtoViewport _output_get 999)))
    (else
      (bind _loadingscreen (Variables|WidgetsRefs|GetLoadingScreen)
        (:then
          (Widget|RemovefromParent _loadingscreen))
        (:else)))))

(fn FShowNotify
  (params (Message :type String))
  (Utilities|FlowControl|Sequence
    (:then_0
      (bind _notify (Variables|WidgetsRefs|GetNotify)
        (:then
          (Widget|RemovefromParent _notify))
        (:else)))
    (:then_1
      (bind _returnvalue (UserInterface|CreateWidget "/Game/Blueprints/Widgets/Game/BP_W_Notify.BP_W_Notify_C" (Variables|Default|GetPlayerOwner) Message))
      (bind _output_get (Variables|WidgetsRefs|SetNotify _returnvalue))
      (UserInterface|Viewport|AddtoViewport _output_get 50))))

(fn FToggleScoreBoard
  (params (Show :type Boolean))
  (if Show
    (bind _scoreboard (Variables|WidgetsRefs|GetScoreboard)
      (:then
        (Utilities|MHIsWidgetVisible _scoreboard
          (:false
            (UserInterface|Viewport|AddtoViewport _scoreboard 100))))
      (:else
        (bind _returnvalue (UserInterface|CreateWidget "/Game/Blueprints/Widgets/Scoreboard/BP_W_ScoreBoard.BP_W_ScoreBoard_C" (Variables|Default|GetPlayerOwner)))
        (bind _output_get (Variables|WidgetsRefs|SetScoreboard _returnvalue))
        (UserInterface|Viewport|AddtoViewport _output_get 100)))
    (else
      (bind _scoreboard_2 (Variables|WidgetsRefs|GetScoreboard)
        (:then
          (Widget|RemovefromParent _scoreboard_2))
        (:else)))))

(fn FToggleRoundFinishScreen
  (params (Show :type Boolean))
  (if Show
    (Variables|WidgetsRefs|GetRoundFinishScreen
      (:then
        (Utilities|MHIsWidgetVisible (Variables|WidgetsRefs|GetRoundFinishScreen)
          (:false
            (UserInterface|Viewport|AddtoViewport (Variables|WidgetsRefs|GetRoundFinishScreen) 0))))
      (:else
        (bind _returnvalue (UserInterface|CreateWidget "/Game/Blueprints/Widgets/Game/BP_W_GameFinishScreen.BP_W_GameFinishScreen_C" (Variables|Default|GetPlayerOwner)))
        (bind _output_get (Variables|WidgetsRefs|SetRoundFinishScreen _returnvalue))
        (UserInterface|Viewport|AddtoViewport _output_get 0)))
    (else
      (bind _roundfinishscreen (Variables|WidgetsRefs|GetRoundFinishScreen)
        (:then
          (Widget|RemovefromParent _roundfinishscreen))
        (:else)))))

(fn FToggleGameChat
  (params (Show :type Boolean))
  (if Show
    (Variables|WidgetsRefs|GetGameChat
      (:then
        (Utilities|MHIsWidgetVisible (Variables|WidgetsRefs|GetGameChat)
          (:false
            (UserInterface|Viewport|AddtoViewport (Variables|WidgetsRefs|GetGameChat) 0))))
      (:else
        (bind _returnvalue (UserInterface|CreateWidget "/Game/Blueprints/Widgets/Chat/BP_W_GameChat.BP_W_GameChat_C" (Variables|Default|GetPlayerOwner)))
        (bind _output_get (Variables|WidgetsRefs|SetGameChat _returnvalue))
        (UserInterface|Viewport|AddtoViewport _output_get 0)))
    (else
      (bind _gamechat (Variables|WidgetsRefs|GetGameChat)
        (:then
          (Widget|RemovefromParent _gamechat))
        (:else)))))