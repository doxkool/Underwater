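; Base player controller for the multiplayer kernel, bridging client input and UI with the server.
; On begin play it fetches host settings through a server RPC and caches them in the local GameInstance for UI.
; Server RPCs relay chat, lobby readiness, pawn destruction and disconnects, with a client RPC ending the session.
; Input toggles the in-game menu, scoreboard and chat through the HUD; debug test keys remain.
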(event Custom|SRV_DestroyPawn
  (bind _returnvalue (Pawn|GetSpectatorPawn))
  ;[1 1 1] Destroy character
  (Utilities|IsValid _returnvalue
    (:Is%20Valid
      (Actor|DestroyActor _returnvalue))
    (:Is%20Not%20Valid
      _))
  (Class|BPIBaseCharacter|IEDestroySelf(Message) (Pawn|GetControlledPawn)))

(event Custom|srv
  (Development|PrintString (Utilities|String|ToString(Integer) (Variables|/Game/Blueprints/Kernel/BP_Kernel_GM.BP_Kernel_GM_C|GetMinPlayersToStart (CallFunction|HKernelGM)))))

(event Custom|CL_SaveHostSettingsInLocalGI
  (params (ServerName :type String) (MinPlayersToStart :type Integer))
  (bind _maingi (CallFunction|HMainGI))
  ;[1 0 0.1247] Save host settings in local GameInstance. We need them for UI
  (Variables|/Game/Blueprints/Kernel/BP_MainGI.BP_MainGI_C|SetServerName _maingi ServerName)
  (Variables|/Game/Blueprints/Kernel/BP_MainGI.BP_MainGI_C|SetMinPlayersToStart _maingi MinPlayersToStart))

(event Custom|SRV_GetHostSettings
  (bind _kernelgm (CallFunction|HKernelGM))
  ;[1 0 0.1247] Get host settings from server
  (CallFunction|CLSaveHostSettingsinLocalGI (Variables|/Game/Blueprints/Kernel/BP_Kernel_GM.BP_Kernel_GM_C|GetServerName _kernelgm) (Variables|/Game/Blueprints/Kernel/BP_Kernel_GM.BP_Kernel_GM_C|GetMinPlayersToStart _kernelgm)))

(event Custom|SRV_Disconnect
  ;[1 1 1] Disconnect
  (CallFunction|IEDestroyControlledPawn)
  (CallFunction|CLDisconnect))

(event Custom|CL_Disconnect
  ;[1 1 1] Disconnect
  (Default|EDestroySessionandGotoMainMenu (CallFunction|HMainGI) self))

(event Custom|srv_5
  ;[1 1 1] for testing. set current time = 2 seconds
  (Variables|/Game/Blueprints/Kernel/BP_Kernel_GS.BP_Kernel_GS_C|SetCurrentTime (CallFunction|HKernelGS) 2))

(event EventEndPlay
  (params (EndPlayReason :type EEndPlayReason%20Enum :default "Destroyed"))
  ;[1 1 1] Disconnect
  (CallFunction|IEDestroyControlledPawn))

(event EventIEDisconnectfromtheServer
  ;[1 1 1] Disconnect
  (CallFunction|SRVDisconnect))

(event EventIEDestroyControlledPawn
  ;[1 1 1] Destroy character
  (CallFunction|SRVDestroyPawn))

(event EventBeginPlay
  ;[1 1 1] Begin play. Load game setting from server - we need them for ui
  (if (Pawn|IsLocalPlayerController)
    (CallFunction|SRVGetHostSettings)))

(event Input|KeyboardEvents|1
  (params (Key :type Key%20Structure))
  (:Pressed
    (CallFunction|Srv)))

(event Input|KeyboardEvents|Add
  (params (Key :type Key%20Structure))
  ;[1 1 1] for testing. set current time = 2 seconds
  (:Pressed
    (CallFunction|Srv5)))

(event Custom|SRV_SendChatMessage
  (params (IsServer :type Boolean) (Message :type String))
  ;[0 0.6122 1] Send chat message
  (Default|MCUpdateGameChat (CallFunction|HKernelGS) IsServer (Variables|/Script/Engine.PlayerState|GetPlayerId (Variables|GetPlayerState)) Message))

(event Custom|SRV_Ready
  ;[1 1 1] Change ready status in lobby
  (bind _asbp_kernel_ps (Utilities|Casting|CastToBP_Kernel_PS (Variables|GetPlayerState)))
  (Variables|/Game/Blueprints/Kernel/BP_Kernel_PS.BP_Kernel_PS_C|SetIsReady _asbp_kernel_ps true)
  (Default|FSTrytoStartLobbyCountdown (CallFunction|HKernelGS)))

(event Custom|SRV_SendLobbyMessage
  (params (Message :type String))
  ;[1 1 1] Send lobby message
  (Default|MCUpdateLobbyChat (CallFunction|HKernelGS) (Variables|/Script/Engine.PlayerState|GetPlayerId (Variables|GetPlayerState)) Message))

(event Input|ActionEvents|InputActionShowScoreboard
  (params (Key :type Key%20Structure))
  (bind _kernelhud (CallFunction|HKernelHUD))
  ;[1 1 1] Show Scoreboard
  (:Pressed
    (if (Utilities|Enum|Equal(Enum) (Variables|/Game/Blueprints/Kernel/BP_Kernel_GS.BP_Kernel_GS_C|GetGlobalState (CallFunction|HKernelGS)) "NewEnumerator17")
      (Default|FToggleGameChat _kernelhud false)
      (Default|FToggleScoreBoard _kernelhud true)))
  (:Released
    (Default|FToggleScoreBoard _kernelhud false)))

(event Input|ActionEvents|InputActionOpenGameChat
  (params (Key :type Key%20Structure))
  (bind _kernelhud (CallFunction|HKernelHUD))
  ;[0 0.6122 1] Open game chat
  (:Pressed
    (if (Utilities|Enum|Equal(Enum) (Variables|/Game/Blueprints/Kernel/BP_Kernel_GS.BP_Kernel_GS_C|GetGlobalState (CallFunction|HKernelGS)) "NewEnumerator17")
      (Default|FToggleGameChat _kernelhud true)
      (Default|EOpenChat (Variables|/Game/Blueprints/Kernel/BP_Kernel_HUD.BP_Kernel_HUD_C|GetGameChat _kernelhud)))))

(event Input|ActionEvents|InputActionOpenIngameMenu
  (params (Key :type Key%20Structure))
  (bind _returnvalue (Game|GetPlayerCharacter 0))
  (bind _returnvalue_2 (Game|GetPlayerCharacter 0))
  ;[1 1 1] Show / hide in-game menu
  (:Pressed
    (bind _isa (Utilities|FlowControl|FlipFlop)
      (:A
        (if _isa
          (Default|FToggleinGameMenu (CallFunction|HKernelHUD) true)
          (Variables|Default|SetbShowMouseCursor true)
          (Utilities|IsValid _returnvalue_2
            (:Is%20Valid
              (Input|DisableInput _returnvalue_2 self)))))
      (:B
        (Default|FToggleinGameMenu (CallFunction|HKernelHUD) false)
        (Variables|/Script/Engine.PlayerController|SetbShowMouseCursor (Game|GetPlayerController 0) false)
        (Utilities|IsValid _returnvalue
          (:Is%20Valid
            (Input|EnableInput _returnvalue self)))))))

(event Input|KeyboardEvents|Z
  (params (Key :type Key%20Structure))
  (bind _returnvalue (Game|GetPlayerCharacter 0))
  (bind _returnvalue_2 (Game|GetPlayerCharacter 0))
  ;[1 1 1] Show / hide in-game menu
  (:Pressed
    (bind _isa (Utilities|FlowControl|FlipFlop)
      (:A
        (if _isa
          (Default|FToggleinGameMenu (CallFunction|HKernelHUD) true)
          (Variables|Default|SetbShowMouseCursor true)
          (Utilities|IsValid _returnvalue_2
            (:Is%20Valid
              (Input|DisableInput _returnvalue_2 self)))))
      (:B
        (Default|FToggleinGameMenu (CallFunction|HKernelHUD) false)
        (Variables|/Script/Engine.PlayerController|SetbShowMouseCursor (Game|GetPlayerController 0) false)
        (Utilities|IsValid _returnvalue
          (:Is%20Valid
            (Input|EnableInput _returnvalue self)))))))

(fn ConstructionScript)