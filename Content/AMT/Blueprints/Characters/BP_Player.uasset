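; Networked player character for a multiplayer game where players repair generators to open the gates.
; Axis and action inputs drive movement, with sprint, crouch and direction values sent to the server.
; A per-tick camera trace finds unrepaired generators; holding Interact runs a HUD progress timeline, then the server repairs and opens gates after enough repairs.
; Point damage feeds the health manager, shows client indicators and triggers multicast ragdoll death with a random broken constraint.
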(event Custom|SRV_Crouch
  (params (crouch :type Boolean))
  ;[1 1 1] Crouch
  (bind _output_get (Variables|State|SetIsCrouching crouch))
  (CallFunction|FSetCrouchSpeed _output_get))

(event Custom|SRV_RepairGenerator
  (bind _kernelgs (CallFunction|HKernelGS))
  (bind _actoryouarelookingat (Variables|Default|GetActorYouAreLookingAt))
  ;[0 0.5744 1] Repair generator
  (Utilities|FlowControl|Sequence
    (:then_0
      (Utilities|IsValid _actoryouarelookingat
        (:Is%20Valid
          (bind _asbp_generator (Utilities|Casting|CastToBP_Generator _actoryouarelookingat))
          (Default|EARepair _asbp_generator))))
    (:then_1
      (Variables|/Game/AMT/Blueprints/Kernel/BP_Kernel_GS.BP_Kernel_GS_C|SetRepairedGenerators _kernelgs (+ (Variables|/Game/AMT/Blueprints/Kernel/BP_Kernel_GS.BP_Kernel_GS_C|GetRepairedGenerators _kernelgs) 1)))
    (:then_2
      (if (>= (Variables|/Game/AMT/Blueprints/Kernel/BP_Kernel_GS.BP_Kernel_GS_C|GetRepairedGenerators (CallFunction|HKernelGS)) 3)
        (bind _outactors (Actor|GetAllActorsOfClass "/Game/AMT/Blueprints/Actors/BP_Gate.BP_Gate_C"))
        (for _array_element _outactors
          (Default|EAOpenGate _array_element)
          (Default|MCSendNotify (CallFunction|HKernelGS) "THE GATES ARE OPEN"))))))

(event Custom|SRV_UpdateDirection
  (params (MoveForward :type Float%20%28single-precision%29) (MoveRight :type Float%20%28single-precision%29) (MoveRightAxisValue :type Float%20%28single-precision%29))
  ;[0 0.978 1] Movement input - WASD
  (Variables|MovementReplication|SetMoveForward MoveForward)
  (Variables|MovementReplication|SetMoveRight MoveRight)
  (Variables|MovementReplication|SetMoveRightAxisValue MoveRightAxisValue))

(event Custom|CL_ShowDamageIndicator
  (params (BulletTraceStart :type Vector))
  ;[0.6172 0 1] Show damage indicator on client
  (bind _returnvalue (UserInterface|CreateWidget "/Game/AMT/Blueprints/Widgets/Game/BP_W_DamageIndicator.BP_W_DamageIndicator_C" (Game|GetPlayerController 0) BulletTraceStart))
  (UserInterface|Viewport|AddtoViewport _returnvalue 0))

(event Custom|SRV_Sprint
  (params (IsSptinting :type Boolean))
  ;[1 1 1] Sprint
  (bind _output_get (Variables|State|SetIsSprinting IsSptinting))
  (CallFunction|FSetSprintSpeed _output_get))

(event Custom|MC_Death
  ;[0.6172 0 1] Multicast death
  (Physics|SetSimulatePhysics (Variables|Character|GetMesh) true)
  (Collision|SetCollisionEnabled (Variables|Collision|GetCapsuleComponent) "NoCollision")
  (Class|SkeletalMeshComponent|BreakConstraint (Variables|Character|GetMesh) "0, 0, 0" "0, 0, 0" (Utilities|Select :Index (Math|Random|RandomInteger 4) :Option%200 "spine_01" :Option%201 "thigh_r" :Option%202 "thigh_l" :Option%203 "upperarm_r" :Option%204 "upperarm_l")))

(event EventTick
  (params (DeltaSeconds :type Float%20%28single-precision%29))
  ;[1 1 1] Tick
  (CallFunction|FSSearchRay))

(event EventIEDestroySelf
  ;[1 1 1] Destroy character
  (Actor|DestroyActor))

(event Game|Damage|EventPointDamage
  (params (Damage :type Float%20%28single-precision%29) (DamageType :type Damage%20Type%20Object%20Reference) (HitLocation :type Vector :default "0, 0, 0") (HitNormal :type Vector :default "0, 0, 0") (HitComponent :type Primitive%20Component%20Object%20Reference) (BoneName :type Name :default "None") (ShotFromDirection :type Vector :default "0, 0, 0") (InstigatedBy :type Controller%20Object%20Reference) (DamageCauser :type Actor%20Object%20Reference) (HitInfo :type Hit%20Result%20Structure%20%28by%20ref%29))
  ;[0.6144 0 1] Point damage
  (if (not (Variables|State|GetIsDead))
    (CallFunction|CLShowDamageIndicator (.TraceStart (Collision|BreakHitResult HitInfo)))
    (bind _isdead (Default|FSApplyDamage (Variables|Default|GetBP_HealthManager) Damage))
    (if _isdead
      (Variables|State|SetIsDead true)
      (Default|FSProcessPlayerDeath (CallFunction|HKernelGM) (Variables|GetPlayerState) (Variables|/Script/Engine.Controller|GetPlayerState InstigatedBy))
      (CallFunction|MCDeath)
      (Actor|SetLifeSpan 5.0))))

(event Input|ActionEvents|InputActionCrouch
  (params (Key :type Key%20Structure :default "None"))
  ;[1 1 1] Crouch
  (:Pressed
    (if (Variables|State|GetIsCrouching)
      (CallFunction|SRVCrouch false)
      (CallFunction|FSetCrouchSpeed false)
      (else
        (CallFunction|SRVCrouch true)
        (CallFunction|FSetCrouchSpeed true)))))

(event Input|ActionEvents|InputActionInteract
  (params (Key :type Key%20Structure :default "None"))
  ;[0 0.4721 1] Interact - repair generator. You can change repair time in timeline
  (:Pressed
    (Utilities|IsValid (Variables|Default|GetActorYouAreLookingAt)
      (:Is%20Valid
        (Utilities|IsValid (CallFunction|HKernelHUD)
          (:Is%20Valid
            (bind _alpha (Timeline|RepairTimeline PlayFromStart)
              (:Update
                (Utilities|IsValid (Variables|Default|GetActorYouAreLookingAt)
                  (:Is%20Valid
                    (bind _returnvalue (Appearance|GetDynamicMaterial (Variables|/Game/AMT/Blueprints/Widgets/Game/BP_W_HUD.BP_W_HUD_C|GetProgressCircle (Variables|/Game/AMT/Blueprints/Kernel/BP_Kernel_HUD.BP_Kernel_HUD_C|GetPlayerHud (CallFunction|HKernelHUD))) :!class /Script/UMG.Image))
                    (Rendering|Material|SetScalarParameterValue _returnvalue (Utilities|Name|MakeLiteralName "Alpha") _alpha :!class /Script/Engine.MaterialInstanceDynamic))
                  (:Is%20Not%20Valid
                    (CallFunction|FResetActionLoader :!label _label))))
              (:Finished
                (CallFunction|SRVRepairGenerator)
                (goto _label))))))
      (:Is%20Not%20Valid
        (CallFunction|FResetActionLoader :!label _label_2))))
  (:Released
    (goto _label_2)))

(event Input|ActionEvents|InputActionSprint
  (params (Key :type Key%20Structure :default "None"))
  ;[1 1 1] Sprint
  (:Pressed
    (CallFunction|SRVCrouch false)
    (CallFunction|SRVSprint true)
    (CallFunction|FSetSprintSpeed true))
  (:Released
    (CallFunction|SRVSprint false)
    (CallFunction|FSetSprintSpeed false)))

(event Input|ActionEvents|InputActionJump
  (params (Key :type Key%20Structure :default "None"))
  ;[0.004949 0.83 1] SPACE - Jump
  (:Pressed
    (Character|Jump))
  (:Released
    (Character|StopJumping)))

(event Input|AxisEvents|InputAxisMoveForward
  (params (AxisValue :type Float%20%28single-precision%29))
  ;[0 0.978 1] Movement input - WASD
  (bind _output_get (Variables|MovementReplication|SetMoveForwardAxisValue AxisValue))
  (Pawn|Input|AddMovementInput (Math|Vector|GetForwardVector (Math|Rotator|MakeRotator 0.0 0.0 (.Yaw (Math|Rotator|BreakRotator (Pawn|GetControlRotation :!class /Script/Engine.Pawn))))) _output_get false)
  (bind (_moveforward _moveright) (CallFunction|FCalculateMovement))
  (CallFunction|SRVUpdateDirection _moveforward _moveright (Variables|MovementReplication|GetMoveRightAxisValue)))

(event Input|AxisEvents|InputAxisMoveRight
  (params (AxisValue :type Float%20%28single-precision%29))
  ;[0 0.978 1] Movement input - WASD
  (bind _output_get (Variables|MovementReplication|SetMoveRightAxisValue AxisValue))
  (Pawn|Input|AddMovementInput (Math|Vector|GetRightVector (Math|Rotator|MakeRotator 0.0 0.0 (.Yaw (Math|Rotator|BreakRotator (Pawn|GetControlRotation :!class /Script/Engine.Pawn))))) _output_get false))

(event Input|AxisEvents|InputAxisLookUp
  (params (AxisValue :type Float%20%28single-precision%29))
  ;[0 1 0.9414] mouse - Look up
  (Pawn|Input|AddControllerPitchInput AxisValue))

(event Input|AxisEvents|InputAxisTurn
  (params (AxisValue :type Float%20%28single-precision%29))
  ;[0 1 0.9414] mouse - Turn
  (Pawn|Input|AddControllerYawInput AxisValue))

(fn ConstructionScript)

(fn FCalculateMovement
  (bind _returnvalue (Transformation|GetActorRotation))
  (bind _returnvalue_2 (Pawn|GetControlRotation :!class /Script/Engine.Pawn))
  (bind _moveforwardaxisvalue (Variables|MovementReplication|GetMoveForwardAxisValue))
  (bind _moverightaxisvalue (Variables|MovementReplication|GetMoveRightAxisValue))
  (bind _returnvalue_3 (Math|Rotator|Delta(Rotator) _returnvalue_2 _returnvalue))
  (bind _yaw (Math|Rotator|BreakRotator _returnvalue_3))
  (bind _returnvalue_4 (- 0.0 _yaw))
  (Utilities|FlowControl|Sequence
    (:then_0
      (bind _output_get (Variables|MovementReplication|SetMoveForward (+ (* _moveforwardaxisvalue (Math|Trig|Cos(Degrees) _yaw)) (* (Math|Trig|Sin(Degrees) _returnvalue_4) _moverightaxisvalue)))))
    (:then_1
      (bind _output_get_2 (Variables|MovementReplication|SetMoveRight (+ (* _moveforwardaxisvalue (Math|Trig|Sin(Degrees) _yaw)) (* (Math|Trig|Cos(Degrees) _returnvalue_4) _moverightaxisvalue))))
      (return _output_get _output_get_2))))

(fn FGetDefaultTrace
  (params (Lenght :type Float%20%28single-precision%29))
  (bind _followcamera (Variables|MyCharacter|GetFollowCamera))
  (bind _returnvalue (Transformation|GetWorldLocation _followcamera))
  (bind _returnvalue_2 (Math|Vector|GetForwardVector _followcamera))
  (return (+ _returnvalue (* _returnvalue_2 3e+02)) (+ _returnvalue (* _returnvalue_2 Lenght))))

(fn OnRepIsDead
  (Networking|SwitchHasAuthority
    (:Authority
      (bind _asbp_kernel_ps (Utilities|Casting|CastToBP_Kernel_PS (Variables|GetPlayerState)))
      (Variables|/Game/AMT/Blueprints/Kernel/BP_Kernel_PS.BP_Kernel_PS_C|SetIsDead _asbp_kernel_ps true))))

(fn FSetSprintSpeed
  (params (Sprintt :type Boolean))
  (bind _charactermovement (Variables|Character|GetCharacterMovement))
  (if Sprintt
    (Variables|/Script/Engine.CharacterMovementComponent|SetMaxWalkSpeed _charactermovement (Variables|Default|GetSprintSpeed))
    (else
      (Variables|/Script/Engine.CharacterMovementComponent|SetMaxWalkSpeed _charactermovement (Variables|Default|GetJogSpeed)))))

(fn FSetCrouchSpeed
  (params (crouch :type Boolean))
  (bind _charactermovement (Variables|Character|GetCharacterMovement))
  (if crouch
    (Variables|/Script/Engine.CharacterMovementComponent|SetMaxWalkSpeed _charactermovement (Variables|Default|GetCrouchSpeed))
    (else
      (Variables|/Script/Engine.CharacterMovementComponent|SetMaxWalkSpeed _charactermovement (Variables|Default|GetJogSpeed)))))

(fn FResetActionLoader
  (Audio|Components|Audio|Stop (Variables|Default|GetRepairTimeline))
  (bind _returnvalue (Appearance|GetDynamicMaterial (Variables|/Game/AMT/Blueprints/Widgets/Game/BP_W_HUD.BP_W_HUD_C|GetProgressCircle (Variables|/Game/AMT/Blueprints/Kernel/BP_Kernel_HUD.BP_Kernel_HUD_C|GetPlayerHud (CallFunction|HKernelHUD))) :!class /Script/UMG.Image))
  (Rendering|Material|SetScalarParameterValue _returnvalue (Utilities|Name|MakeLiteralName "Alpha") 0.0 :!class /Script/Engine.MaterialInstanceDynamic))

(fn FSSearchRay
  (bind _followcamera (Variables|MyCharacter|GetFollowCamera))
  (bind _returnvalue (Transformation|GetWorldLocation _followcamera))
  (bind (_outhit _returnvalue_2) (Collision|LineTraceByChannel _returnvalue (+ _returnvalue (* (Math|Vector|GetForwardVector _followcamera) 5e+02)) "TraceTypeQuery1" false 0 "None"))
  (if _returnvalue_2
    (bind _asbp_generator (Utilities|Casting|CastToBP_Generator (.HitActor (Collision|BreakHitResult _outhit)))
      (:then
        (if (not (Variables|/Game/AMT/Blueprints/Actors/BP_Generator.BP_Generator_C|GetIsRepaired _asbp_generator))
          (if (!= (Variables|Default|GetActorYouAreLookingAt) _asbp_generator)
            (Variables|Default|SetActorYouAreLookingAt _asbp_generator))
          (else
            (Utilities|IsValid (Variables|Default|GetActorYouAreLookingAt)
              (:Is%20Valid
                (Variables|Default|SetActorYouAreLookingAt 0))))))
      (:CastFailed
        (Utilities|IsValid (Variables|Default|GetActorYouAreLookingAt) :!label _label
          (:Is%20Valid
            (Variables|Default|SetActorYouAreLookingAt 0)))))
    (else
      (goto _label))))

(fn IFGetFollowCamera
  (return (Variables|MyCharacter|GetFollowCamera)))

(fn IFGetHealth
  (return (Variables|/Game/AMT/Blueprints/Characters/BP_HealthManager.BP_HealthManager_C|GetHealth (Variables|Default|GetBP_HealthManager))))

(fn IFIsDead
  (return (Variables|State|GetIsDead)))

(fn IFSetHealth
  (params (NewHealth :type Float%20%28single-precision%29))
  (bind _output_get (Variables|/Game/AMT/Blueprints/Characters/BP_HealthManager.BP_HealthManager_C|SetHealth (Variables|Default|GetBP_HealthManager) NewHealth))
  (return _output_get))