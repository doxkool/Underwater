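; BP_Monster is a player-controlled, networked monster character with mouse look, WASD movement, jump, sprint and a melee attack.
; On authority it spawns a melee weapon on the right-hand socket; attacks trigger its swing via a server event and multicast the montage, gated by animation length.
; Server events also receive sprint state and control-rotation-relative movement values.
; Interface functions expose camera, death state and health manager, and IsDead replication writes to the PlayerState on authority.
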(event Custom|SRV_MeleeAttack
  ;[0.8438 0 0.02777] LMB - melee attack
  (Default|EASwing (Variables|MeleeAttack|GetMeleeWeapon))
  (CallFunction|MCMeleeAttack))

(event Custom|SRV_UpdateDirection
  (params (MoveForward :type Float%20%28single-precision%29) (MoveRight :type Float%20%28single-precision%29) (MoveRightAxisValue :type Float%20%28single-precision%29))
  ;[0 0.978 1] Movement input - WASD
  (Variables|MovementReplication|SetMoveForward MoveForward)
  (Variables|MovementReplication|SetMoveRight MoveRight)
  (bind _output_get (Variables|MovementReplication|SetMoveRightAxisValue MoveRightAxisValue))
  (if (!= _output_get 0.0)
    (Variables|AnimationState|SetIsSprinting false)))

(event Custom|MC_MeleeAttack
  ;[0.8438 0 0.02777] LMB - melee attack
  (Animation|Montage|PlayMontage (Variables|Character|GetMesh) (Variables|MeleeAttack|GetAttackAnim)))

(event Custom|SRV_Sprint
  (params (IsSptinting :type Boolean))
  ;[0.9361 0.1939 1] SHIFT - Sprint
  (bind _output_get (Variables|AnimationState|SetIsSprinting IsSptinting))
  (CallFunction|FSetSprintSpeed _output_get))

(event EventBeginPlay
  ;[1 1 1] Begin play. Create melee weapon
  (Networking|SwitchHasAuthority
    (:Authority
      (CallFunction|FSCreateMeleeWeapon))))

(event EventIEDestroySelf
  ;[1 0 0.05349] Destroy character and his weapons
  (Actor|DestroyActor (Variables|MeleeAttack|GetMeleeWeapon))
  (Actor|DestroyActor))

(event Input|ActionEvents|InputActionSprint
  (params (Key :type Key%20Structure))
  ;[0.9361 0.1939 1] SHIFT - Sprint
  (:Pressed
    (CallFunction|SRVSprint true))
  (:Released
    (CallFunction|SRVSprint false)))

(event Input|ActionEvents|InputActionJump
  (params (Key :type Key%20Structure))
  ;[0.9361 0.1939 1] SPACE - Jump
  (:Pressed
    (Character|Jump))
  (:Released
    (Character|StopJumping)))

(event Input|ActionEvents|InputActionLMB
  (params (Key :type Key%20Structure))
  ;[0.8438 0 0.02777] LMB - melee attack
  (:Pressed
    (if (not (Variables|MeleeAttack|GetIsMeleeActive))
      (Variables|MeleeAttack|SetIsMeleeActive true)
      (CallFunction|SRVMeleeAttack)
      (bind _returnvalue (Animation|GetPlayLength (Variables|MeleeAttack|GetAttackAnim)))
      (Utilities|FlowControl|Delay _returnvalue)
      (Variables|MeleeAttack|SetIsMeleeActive false))))

(event Input|AxisEvents|InputAxisMoveForward
  (params (AxisValue :type Float%20%28single-precision%29))
  ;[0 0.978 1] Movement input - WASD
  (bind _output_get (Variables|MovementReplication|SetMoveForwardAxisValue AxisValue))
  (Pawn|Input|AddMovementInput (Math|Vector|GetForwardVector (Math|Rotator|MakeRotator 0.0 0.0 (.Yaw (Math|Rotator|BreakRotator (Pawn|GetControlRotation :!class /Script/Engine.Pawn))))) _output_get false)
  (bind (_moveforward _moveright) (CallFunction|FCalculateMovement))
  (CallFunction|SRVUpdateDirection _moveforward _moveright (Variables|MovementReplication|GetMoveRightAxisValue)))

(event Input|AxisEvents|InputAxisMoveRight
  (params (AxisValue :type Float%20%28single-precision%29))
  ;[0 0.978 1] Movement input - WASD
  (bind _output_get (Variables|MovementReplication|SetMoveRightAxisValue AxisValue))
  (Pawn|Input|AddMovementInput (Math|Vector|GetRightVector (Math|Rotator|MakeRotator 0.0 0.0 (.Yaw (Math|Rotator|BreakRotator (Pawn|GetControlRotation :!class /Script/Engine.Pawn))))) _output_get false))

(event Input|AxisEvents|InputAxisLookUp
  (params (AxisValue :type Float%20%28single-precision%29))
  ;[0 1 0.9414] mouse - Look up
  (Pawn|Input|AddControllerPitchInput AxisValue))

(event Input|AxisEvents|InputAxisTurn
  (params (AxisValue :type Float%20%28single-precision%29))
  ;[0 1 0.9414] mouse - Turn
  (Pawn|Input|AddControllerYawInput AxisValue))

(fn ConstructionScript)

(fn FCalculateMovement
  (bind _returnvalue (Transformation|GetActorRotation))
  (bind _returnvalue_2 (Pawn|GetControlRotation :!class /Script/Engine.Pawn))
  (bind _moveforwardaxisvalue (Variables|MovementReplication|GetMoveForwardAxisValue))
  (bind _moverightaxisvalue (Variables|MovementReplication|GetMoveRightAxisValue))
  (bind _returnvalue_3 (Math|Rotator|Delta(Rotator) _returnvalue_2 _returnvalue))
  (bind _yaw (Math|Rotator|BreakRotator _returnvalue_3))
  (bind _returnvalue_4 (- 0.0 _yaw))
  (Utilities|FlowControl|Sequence
    (:then_0
      (bind _output_get (Variables|MovementReplication|SetMoveForward (+ (* _moveforwardaxisvalue (Math|Trig|Cos(Degrees) _yaw)) (* (Math|Trig|Sin(Degrees) _returnvalue_4) _moverightaxisvalue)))))
    (:then_1
      (bind _output_get_2 (Variables|MovementReplication|SetMoveRight (+ (* _moveforwardaxisvalue (Math|Trig|Sin(Degrees) _yaw)) (* (Math|Trig|Cos(Degrees) _returnvalue_4) _moverightaxisvalue))))
      (return _output_get _output_get_2))))

(fn FSetSprintSpeed
  (params (Sprint :type Boolean))
  (bind _charactermovement (Variables|Character|GetCharacterMovement))
  (if Sprint
    (Variables|/Script/Engine.CharacterMovementComponent|SetMaxWalkSpeed _charactermovement (Variables|MovementSpeedSettings|GetSprintSpeed))
    (else
      (Variables|/Script/Engine.CharacterMovementComponent|SetMaxWalkSpeed _charactermovement (Variables|MovementSpeedSettings|GetJogSpeed)))))

(fn FStopSprint
  (if (Variables|AnimationState|GetIsSprinting)
    (CallFunction|FSetSprintSpeed false)
    (CallFunction|SRVSprint false)))

(fn OnRepIsDead
  (Networking|SwitchHasAuthority
    (:Authority
      (bind _asbp_kernel_ps (Utilities|Casting|CastToBP_Kernel_PS (Variables|GetPlayerState)))
      (Variables|/Game/AMT/Blueprints/Kernel/BP_Kernel_PS.BP_Kernel_PS_C|SetIsDead _asbp_kernel_ps (Variables|State|GetIsDead)))))

(fn FSCreateMeleeWeapon
  (bind _self self)
  (bind _returnvalue (Game|SpawnActorfromClass "/Game/AMT/Blueprints/Weapons/BP_MeleeWeapon.BP_MeleeWeapon_C" (Transformation|GetSocketTransform (Variables|Character|GetMesh) "rhand" "RTS_World") "Undefined" self 0))
  (bind _output_get (Variables|MeleeAttack|SetMeleeWeapon _returnvalue))
  (Transformation|AttachComponentToComponent _output_get (Variables|Character|GetMesh) "rhand" "SnapToTarget" "SnapToTarget" "SnapToTarget" true)
  (Actor|SetOwner (Variables|MeleeAttack|GetMeleeWeapon) _self)
  (Variables|/Game/AMT/Blueprints/Weapons/BP_MeleeWeapon.BP_MeleeWeapon_C|SetOwnerCharacter (Variables|MeleeAttack|GetMeleeWeapon) _self))

(fn IFGetFollowCamera
  (return (Variables|MyCharacter|GetFollowCamera)))

(fn IFGetHealth
  (return (Variables|/Game/AMT/Blueprints/Characters/BP_HealthManager.BP_HealthManager_C|GetHealth (Variables|Default|GetBP_HealthManager))))

(fn IFIsDead
  (return (Variables|State|GetIsDead)))

(fn IFSetHealth
  (params (NewHealth :type Float%20%28single-precision%29))
  (bind _output_get (Variables|/Game/AMT/Blueprints/Characters/BP_HealthManager.BP_HealthManager_C|SetHealth (Variables|Default|GetBP_HealthManager) NewHealth))
  (return _output_get))