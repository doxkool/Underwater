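; Melee weapon actor that damages Characters its swing passes through, using swept-point line traces instead of collision overlaps.
; On BeginPlay it spaces hidden boxes along Z between top and bottom markers as trace points.
; During the attack animation, a gated Delay loop traces between each box's current and previous location to catch fast swings.
; Each Character except the owner takes point damage once per swing, with a multicast blood effect.
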(event Custom|MC_BloodEffect
  (params (Location :type Vector))
  ;[1 1 1] multicast blood effect
  (Effects|SpawnEmitteratLocation "/Game/AMT/DemoContent/BloodHitEffect/PS_body_bullet_impact.PS_body_bullet_impact" Location "0, 0, 0" "3.000000,3.000000,3.000000"))

(event Custom|EA_WeaponSwing
  ;[1 0.07402 0] Swing
  (Utilities|FlowControl|Sequence
    (:then_0
      (goto _label Open))
    (:then_1
      (Utilities|FlowControl|Gate false :!label _label
        (:Exit
          (Utilities|FlowControl|Sequence
            (:then_0
              (if (Variables|State|GetIsMeleeSwing)
                (bind (_array_element _array_index) (Utilities|Array|ForEachLoopwithBreak (Variables|Meleetrace|GetMeleeTraceBoxes))
                  (:LoopBody
                    (bind _outhits (Collision|MultiLineTraceByChannel (Transformation|GetWorldLocation _array_element) (Utilities|Array|Get(acopy) (Variables|Meleetrace|GetMeleeTracesStartLocations) _array_index) "TraceTypeQuery3" false (Variables|State|GetAlreadyHitActors) "None"))
                    (for _array_element_2 _outhits
                      (bind _output_get (Variables|State|SetLastHit _array_element_2))
                      (if (Info|FCanHitActor (.bBlockingHit (Collision|BreakHitResult _output_get)) (.HitActor (Collision|BreakHitResult _output_get)))
                        (ApplyingDamage|FSTrytoApplyDamage (.HitActor (Collision|BreakHitResult _output_get)))))
                    (Utilities|Array|SetArrayElem (Variables|Meleetrace|GetMeleeTracesStartLocations) _array_index (Transformation|GetWorldLocation _array_element))))
                (else
                  (goto _label Close))))
            (:then_1
              (Utilities|FlowControl|Delay 0.01)
              (goto _label))))))))

(event Custom|EA_Swing
  ;[0 1 0.9539] Attack
  (if (not (Variables|State|GetIsMeleeSwing))
    (Variables|State|SetIsMeleeSwing true)
    (Meleetrace|FUpdateMeleeBoxesLocations)
    (CallFunction|EAWeaponSwing)
    ;;[1 1 1] Wait for swing animation end
    (Utilities|FlowControl|Delay (Variables|/Script/Engine.AnimSequenceBase|GetSequenceLength (Variables|Settings|GetAttackAnimation)))
    (Variables|State|SetIsMeleeSwing false)
    ;;[1 1 1] Clear hit actors
    (Utilities|Array|Clear (Variables|State|GetAlreadyHitActors))
    (Utilities|Array|Clear (Variables|State|GetHitActors))))

(event EventBeginPlay
  ;[1 0 0] BeginPlay - Generate melee trace boxes
  (Meleetrace|FGenerateMeleeTraceBoxes))

(fn ConstructionScript
  (|CallParentFunction))

(fn FGenerateMeleeTraceBoxes
  (Meleetrace|FCalculateOffsetBetweenMeleeBoxes)
  ;[1 1 1] Delete this if you don't want to use top and bottom melee trace boxes
  (Utilities|Array|Add (Variables|Meleetrace|GetMeleeTraceBoxes) (Variables|Default|GetTopMeleeTraceBox))
  (for _index (range 1 (Variables|Meleetrace|GetTracesPerSwing))
    (bind _returnvalue (AddComponent|AddBoxComponent false (Meleetrace|FCalculateMeleeBoxesSpawnOffset _index)))
    (Utilities|Array|Add (Variables|Meleetrace|GetMeleeTraceBoxes) _returnvalue)
    (Development|SetHiddeninGame _returnvalue true false)
    (Transformation|AttachComponentToComponent _returnvalue (Variables|Default|GetWeaponSK) "None" "KeepRelative" "KeepRelative" "KeepRelative" true))
  (Utilities|Array|Add (Variables|Meleetrace|GetMeleeTraceBoxes) (Variables|Default|GetBottomMeleeTraceBox))
  (Meleetrace|FSaveMeleeTraceBoxesLocations))

(fn FSaveMeleeTraceBoxesLocations
  (for _array_element (Variables|Meleetrace|GetMeleeTraceBoxes)
    (Utilities|Array|Add (Variables|Meleetrace|GetMeleeTracesStartLocations) (Transformation|GetWorldLocation _array_element))))

(fn FCalculateMeleeBoxesSpawnOffset
  (params (LoopIndex :type Integer))
  (bind _bottommeleetracebox (Variables|Default|GetBottomMeleeTraceBox))
  (bind _returnvalue (Transformation|GetRelativeTransform _bottommeleetracebox))
  (return (Math|Transform|MakeTransform (Math|Vector|MakeVector (.x (.location _returnvalue)) (.y (.location _returnvalue)) (+ (* LoopIndex (Variables|Meleetrace|GetOffsetBetweenMeleeBoxes)) (.z (.location _returnvalue)))) (.rotation _returnvalue) (.scale _returnvalue))))

(fn FUpdateMeleeBoxesLocations
  (for (_array_element _array_index) (Variables|Meleetrace|GetMeleeTraceBoxes)
    (Utilities|Array|SetArrayElem (Variables|Meleetrace|GetMeleeTracesStartLocations) _array_index (Transformation|GetWorldLocation _array_element))))

(fn FCanHitActor
  (params (WasHit :type Boolean) (HitActor :type Actor%20Object%20Reference))
  (bind _hitactors (Variables|State|GetHitActors))
  (bind _alreadyhitactors (Variables|State|GetAlreadyHitActors))
  (bind _output_get (LocalVariables|SetHitActor_L HitActor))
  (return (Math|Boolean|ANDBoolean WasHit (!= _output_get (Components|GetOwner)) (not (Utilities|Array|IsValidIndex _hitactors (Utilities|Array|FindItem _hitactors (LocalVariables|GetHitActor_L)))) (not (Utilities|Array|IsValidIndex _alreadyhitactors (Utilities|Array|FindItem _alreadyhitactors (LocalVariables|GetHitActor_L)))))))

(fn FSTrytoApplyDamage
  (params (HitActor :type Actor%20Object%20Reference%20%28by%20ref%29))
  (bind _hitactors (Variables|State|GetHitActors))
  (bind _lasthit (Variables|State|GetLastHit))
  (bind _alreadyhitactors (Variables|State|GetAlreadyHitActors))
  (bind (_bblockinghit _binitialoverlap _time _distance _location _impactpoint _normal _impactnormal _physmat _hitactor _hitcomponent _hitbonename _hititem _faceindex _tracestart) (Collision|BreakHitResult _lasthit))
  (Utilities|IsValid (Variables|State|GetOwnerCharacter)
    (:Is%20Valid
      (bind _output_get (LocalVariables|SetHitActor_L HitActor))
      (bind _ascharacter (Utilities|Casting|CastToCharacter _output_get))
      (Utilities|Array|AddUnique _hitactors _ascharacter)
      (if (Utilities|Array|IsValidIndex _hitactors (Utilities|Array|FindItem _hitactors (LocalVariables|GetHitActor_L)))
        (for _array_element (Variables|State|GetHitActors)
          (if (not (Utilities|Array|IsValidIndex _alreadyhitactors (Utilities|Array|FindItem _alreadyhitactors _array_element)))
            (Game|Damage|ApplyPointDamage _array_element (Variables|Settings|GetDamage) _tracestart _lasthit (Game|GetInstigatorController (Variables|State|GetOwnerCharacter)) self)
            (Utilities|Array|AddUnique (Variables|State|GetAlreadyHitActors) _array_element)
            (CallFunction|MCBloodEffect _location)))))))

(fn FCalculateOffsetBetweenMeleeBoxes
  (Variables|Meleetrace|SetOffsetBetweenMeleeBoxes (.z (/ (- (Variables|/Script/Engine.SceneComponent|GetRelativeLocation (Variables|Default|GetTopMeleeTraceBox)) (Variables|/Script/Engine.SceneComponent|GetRelativeLocation (Variables|Default|GetBottomMeleeTraceBox))) (Math|Vector|MakeVector 1.0 1.0 (Math|Conversions|ToFloat(Integer) (+ (Variables|Meleetrace|GetTracesPerSwing) 1)))))))