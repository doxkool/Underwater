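; BP_Kernel_PS is the player state for a round-based monster game, tracking readiness, death and monster turns.
; On the authority it binds to GameState dispatchers to reset flags on lobby state and record monster turns when a round finishes.
; Players joining during Play Time start dead as spectators.
; Death spawns and possesses an observer pawn during play, then switches the client to the observer HUD.
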(event Custom|EA_ResetStats
  ;[1 1 1] BEGIN PLAY
  (Variables|State|SetIsDead false)
  (Variables|State|SetIsReady false))

(event Custom|EA_OnDeath
  ;[1 1 1] On death
  (CallFunction|FSSpawnObserverPawn)
  (CallFunction|CLonDeath))

(event Custom|EA_UpdateMonsterState
  ;[1 1 1] BEGIN PLAY
  (if (Variables|State|GetIsMonster)
    (Variables|State|SetPlayedAsMonster true)))

(event Custom|CL_OnDeath
  (bind _kernelhud (CallFunction|HKernelHUD))
  ;[1 1 1] On death
  (Utilities|IsValid _kernelhud
    (:Is%20Valid
      (Default|FRemoveAll _kernelhud)
      (Default|FToggleOserverHud _kernelhud true))))

(event EventBeginPlay
  (bind _kernelgs (CallFunction|HKernelGS))
  ;[1 1 1] BEGIN PLAY
  (Networking|SwitchHasAuthority
    (:Authority
      (EventDispatchers|BindEventtoDLobbyState _kernelgs (delegate Custom|EA_ResetStats))
      (EventDispatchers|BindEventtoDRoundFinish _kernelgs (delegate Custom|EA_UpdateMonsterState))
      ;;[1 1 1] If player connects during play time he must be dead, because he can only spectate. He will be able to play in the next round
      (switch Utilities|FlowControl|Switch|SwitchonE_GlobalState (Variables|/Game/AMT/Blueprints/Kernel/BP_Kernel_GS.BP_Kernel_GS_C|GetGlobalState (CallFunction|HKernelGS))
        (:NewEnumerator17
          (Variables|State|SetIsDead true))))))

(fn ConstructionScript)

(fn FSSpawnObserverPawn
  (if (Utilities|Enum|Equal(Enum) (Variables|/Game/AMT/Blueprints/Kernel/BP_Kernel_GS.BP_Kernel_GS_C|GetGlobalState (CallFunction|HKernelGS)) "NewEnumerator17")
    (bind _returnvalue (Game|SpawnActorfromClass (Variables|Config|GetObserverClass) (Math|Transform|MakeTransform "0, 0,1000.000000" "0, 0, 0" "1,1,1") "Undefined" 0 0))
    (Pawn|Possess (.AsPlayer%20Controller (Utilities|Casting|CastToPlayerController (Components|GetOwner))) _returnvalue)))

(fn FSIsCurrentMonster
  (return (and (Variables|State|GetIsMonster) (not (Variables|State|GetPlayedAsMonster)))))

(fn FSCanbeMonster
  (return (and (not (Variables|State|GetIsMonster)) (not (Variables|State|GetPlayedAsMonster)))))