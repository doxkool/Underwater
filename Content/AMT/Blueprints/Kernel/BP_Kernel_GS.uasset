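; Game state for a monster-versus-players match that drives the round cycle from start delay through lobby, round start, play time and finish.
; Setting GlobalState fires its OnRep, where the server restarts a one-second countdown and multicasts the change to event dispatchers.
; The lobby timer waits for enough players and shortens when all are ready.
; Also relays chat, kill feed and notifications, and decides the winner from survivors, generators and escape.
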(event Custom|MC_OnGlobalStateChange
  (params (NewGlobalState :type E_GlobalState%20Enum :default "NewEnumerator23"))
  ;[1 0 0.3256] Multicast current state -> call event dispatcher on clients
  (switch Utilities|FlowControl|Switch|SwitchonE_GlobalState NewGlobalState
    (:NewEnumerator23
      (Default|CallDGameStartDelay))
    (:NewEnumerator29
      (Default|CallDLobbyState))
    (:NewEnumerator28
      (Default|CallDRoundStart))
    (:NewEnumerator17
      (Default|CallDPlayTime))
    (:NewEnumerator27
      (Default|CallDRoundFinish))))

(event Custom|MC_SendNotify
  (params (Message :type String))
  ;[1 1 1] Send notification for all
  (Default|CallDNotify Message))

(event Custom|MC_UpdateKillFeed
  (params (KillerId :type Integer) (VictimId :type Integer))
  ;[0 0.8709 1] Update kills log
  (Default|CallDUpdateKillFeed KillerId VictimId))

(event Custom|EA_FinishPlayTime
  ;[1 0 0.0759] Finish play time
  (Utilities|FlowControl|Delay 1.0)
  (Variables|CurrentState|SetGlobalState "NewEnumerator27"))

(event Custom|MC_UpdateGameChat
  (params (IsServer :type Boolean) (SenderId :type Integer) (Message :type String))
  ;[0 0.8709 1] Update game chat
  (Default|CallDUpdateGameChat IsServer SenderId Message))

(event Custom|MC_UpdateLobbyChat
  (params (PlayerId :type Integer) (Message :type String))
  ;[0 0.8706 1] Update lobby chat
  (Default|CallDUpdateLobbyChat PlayerId Message))

(event EventBeginPlay
  ;[1 0.7631 0] BEGIN PLAY
  (Networking|SwitchHasAuthority
    (:Authority
      ;;[1 0 0] It starts main timer. OnRep_GlobalState.
      (Variables|CurrentState|SetGlobalState "NewEnumerator23"))))

(fn ConstructionScript)

(fn FGetAlivePlayers
  (LocalVariables|SetAlivePlayers_L 0)
  (for _array_element (Variables|Default|GetPlayerArray)
    (bind _asbp_kernel_ps (Utilities|Casting|CastToBP_Kernel_PS _array_element))
    (if (and (not (Variables|/Game/AMT/Blueprints/Kernel/BP_Kernel_PS.BP_Kernel_PS_C|GetIsDead _asbp_kernel_ps)) (not (Default|FSIsCurrentMonster _asbp_kernel_ps)))
      (LocalVariables|SetAlivePlayers_L (+ (LocalVariables|GetAlivePlayers_L) 1))))
  (return (LocalVariables|GetAlivePlayers_L)))

(fn FGetTotalPlayers
  (return (Utilities|Array|Length (Variables|Default|GetPlayerArray))))

(fn FSDecreaseTime
  (bind _output_get (Variables|CurrentState|SetCurrentTime (- (Variables|CurrentState|GetCurrentTime) 1)))
  (return (<= _output_get 0)))

(fn FSMainTimer
  (switch Utilities|FlowControl|Switch|SwitchonE_GlobalState (Variables|CurrentState|GetGlobalState)
    (:NewEnumerator23
      (bind _istimeover (MainTimer|FSDecreaseTime :!label _label))
      (if _istimeover
        (MainTimer|FSStopMainTimer)
        (Kernel|FSDefineNextGlobalState)))
    (:NewEnumerator29
      ;[1 1 1] If there are not enought players do not update lobby time
      (if (>= (TotalPlayersQty|FGetTotalPlayers) (Variables|/Game/AMT/Blueprints/Kernel/BP_Kernel_GM.BP_Kernel_GM_C|GetMinPlayersToStart (CallFunction|HKernelGM)))
        (goto _label)
        (else
          (Variables|CurrentState|SetCurrentTime (Variables|TimeSettings|GetLobbyTimeS)))))
    (:NewEnumerator28
      (goto _label))
    (:NewEnumerator17
      (goto _label))
    (:NewEnumerator27
      (goto _label))))

(fn FSStartMainTimer
  (params (NewTime :type Integer))
  (Networking|SwitchHasAuthority
    (:Authority
      (MainTimer|FSStopMainTimer)
      (Variables|CurrentState|SetCurrentTime NewTime)
      (bind _returnvalue (Utilities|Time|SetTimerbyFunctionName 0 "FS_MainTimer" 1.0 true))
      (Variables|Timers|SetMainTimer _returnvalue))))

(fn FSStopMainTimer
  (Utilities|Time|ClearandInvalidateTimerbyHandle (Variables|Timers|GetMainTimer)))

(fn OnRepGlobalState
  (Networking|SwitchHasAuthority
    (:Authority
      (MainTimer|FSStopMainTimer)
      (CallFunction|MConGlobalStateChange (Variables|CurrentState|GetGlobalState))
      (switch Utilities|FlowControl|Switch|SwitchonE_GlobalState (Variables|CurrentState|GetGlobalState)
        (:NewEnumerator23
          (MainTimer|FSStartMainTimer (Variables|TimeSettings|GetGameStartDelayS)))
        (:NewEnumerator29
          (MainTimer|FSStartMainTimer (Variables|TimeSettings|GetLobbyTimeS)))
        (:NewEnumerator28
          (MainTimer|FSStartMainTimer (Variables|TimeSettings|GetRoundStartTimeS)))
        (:NewEnumerator17
          (MainTimer|FSStartMainTimer (Variables|TimeSettings|GetPlayTimeS)))
        (:NewEnumerator27
          (MainTimer|FSStartMainTimer (Variables|TimeSettings|GetRoundFinishTimeS)))))))

(fn FSDefineNextGlobalState
  (switch Utilities|FlowControl|Switch|SwitchonE_GlobalState (Variables|CurrentState|GetGlobalState)
    (:NewEnumerator23
      (Variables|CurrentState|SetRepairedGenerators 0)
      (Variables|CurrentState|SetPlayersEscaped false)
      (Variables|CurrentState|SetGlobalState "NewEnumerator29"))
    (:NewEnumerator29
      (Variables|CurrentState|SetGlobalState "NewEnumerator28"))
    (:NewEnumerator28
      (Variables|CurrentState|SetGlobalState "NewEnumerator17"))
    (:NewEnumerator17
      (Variables|CurrentState|SetGlobalState "NewEnumerator27"))
    (:NewEnumerator27
      (Variables|CurrentState|SetGlobalState "NewEnumerator23"))))

(fn FGetWinner
  (if (Math|Boolean|ORBoolean (<= (AlivePlayers|FGetAlivePlayers) 0) (< (Variables|CurrentState|GetRepairedGenerators) 3) (not (Variables|CurrentState|GetPlayersEscaped)))
    (return "MONSTER")
    (else
      (return "PLAYERS"))))

(fn FSTrytoStartLobbyCountdown
  (for _array_element (Variables|Default|GetPlayerArray)
    (bind _asbp_kernel_ps (Utilities|Casting|CastToBP_Kernel_PS _array_element))
    (if (not (Variables|/Game/AMT/Blueprints/Kernel/BP_Kernel_PS.BP_Kernel_PS_C|GetIsReady _asbp_kernel_ps))
      (return)))
  (if (and (Utilities|Enum|Equal(Enum) (Variables|CurrentState|GetGlobalState) "NewEnumerator29") (> (Variables|CurrentState|GetCurrentTime) 3))
    (Variables|CurrentState|SetCurrentTime 3)))