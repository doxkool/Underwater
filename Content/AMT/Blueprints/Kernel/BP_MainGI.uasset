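; Game instance that manages multiplayer session lifecycle and connection errors.
; Session creation fires a destroy without waiting, then creates a session and opens the requested level with options on success, printing an error on failure.
; Destroy-and-return opens MainMenu both immediately and again on destroy success.
; Travel and network errors toggle the main menu HUD's network error display on when that HUD is valid.
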(event Custom|E_CreateSession
  (params (PublicConnections :type Integer) (bUseLAN :type Boolean) (LevelName :type Name) (Options :type String))
  ;[1 1 1] Create session
  (CallFunction|EDestroySession)
  (|Session (Game|GetPlayerController 0) PublicConnections bUseLAN
    (:OnSuccess
      (Game|OpenLevel(byName) LevelName true Options))
    (:OnFailure
      (Development|PrintString "SESSION CREATION ERROR" true true "(R=0.000000,G=0.660000,B=1.000000,A=1.000000)" 22.0))))

(event Custom|E_DestroySession
  ;[1 1 1] Destroy session
  (|DestroySession (Game|GetPlayerController 0)))

(event Custom|E_DestroySessionAndGoToMainMenu
  (params (PlayerController :type Player%20Controller%20Object%20Reference))
  ;[1 1 1] Destroy session
  (|DestroySession PlayerController
    (:then
      _)
    (:OnSuccess
      _))
  (Game|OpenLevel(byName) "MainMenu"))

(event EventHandleTravelError
  (params (FailureType :type ETravelFailure%20Enum :default "NoLevel"))
  (bind _mainmenuhud (CallFunction|HMainMenuHUD))
  ;[1 0 0] Travel Error
  (Utilities|IsValid _mainmenuhud
    (:Is%20Valid
      (Default|FToggleNetworkError _mainmenuhud true))))

(event EventHandleNetworkError
  (params (FailureType :type ENetworkFailure%20Enum :default "NetDriverAlreadyExists") (bIsServer :type Boolean))
  (bind _mainmenuhud (CallFunction|HMainMenuHUD))
  ;[1 0 0] Network Error
  (Utilities|IsValid _mainmenuhud
    (:Is%20Valid
      (Default|FToggleNetworkError _mainmenuhud true))))