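; Game mode for a monster-versus-players multiplayer round game, handling settings, logins, logouts and spawning.
; Settings come from the dedicated-server command line or host's GameInstance; PostLogin also initializes them because it can precede BeginPlay (UE-27284).
; GameState delegates drive monster rotation, role-based spawning and round-end pawn destruction.
; Late joiners spawn or observe by phase; deaths and departures can end play time.
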(event Custom|EA_RoundStart
  ;[1 1 1] Round start - spawn all players
  (PlayerRespawn|FSSpawnAllPlayers))

(event Custom|E_InitSettings
  ;[1 0.5159 0.0913] INIT SETTINGS
  (if (not (Variables|Config|GetWasInitSettingsSet))
    (Utilities|FlowControl|Sequence
      (:then_0
        (if (Networking|IsDedicatedServer)
          (InitSettings|FSSetGameModeSettingsforDedicatedServer)
          (else
            ;;[1 1 1 1 15] Get host game settings from MainGI
            (InitSettings|FSSetHostGameSettings)))
        ;;[1 1 1] Check and set some default values to avoid errors
        (InitSettings|FCheckHostSettings))
      (:then_1
        (Variables|Config|SetWasInitSettingsSet true)))))

(event Custom|EA_lobby
  ;[1 1 1] Select player to be a monster
  (Monster|FSMakeRandomPlayerMonster))

(event Custom|EA_FinishRound
  ;[1 1 1] round finish - destroy all players
  (Players|FSDestroyAllPlayers))

(event EventBeginPlay
  ;[1 0 0] BEGIN PLAY
  (Utilities|FlowControl|Sequence
    (:then_0
      (Utilities|IsValid (CallFunction|HKernelGS)
        (:Is%20Valid
          _)
        (:Is%20Not%20Valid
          (Utilities|FlowControl|Delay 0.2)))
      (Utilities|FlowControl|Sequence
        (:then_0
          ;[1 1 1] Select player to be a monster
          (EventDispatchers|BindEventtoDLobbyState (CallFunction|HKernelGS) (delegate Custom|EA_lobby)))
        (:then_1
          ;[1 1 1] Round start - spawn all players
          (EventDispatchers|BindEventtoDRoundStart (CallFunction|HKernelGS) (delegate Custom|EA_RoundStart)))
        (:then_2
          ;[1 1 1] round finish - destroy all players
          (EventDispatchers|BindEventtoDRoundFinish (CallFunction|HKernelGS) (delegate Custom|EA_FinishRound)))))
    (:then_1
      (CallFunction|EInitSettings))))

(event EventPostLogin
  (params (NewPlayer :type Player%20Controller%20Object%20Reference))
  ;[0 0.1238 1] LogIn event.
  ; Since OnPostLogin event can be called before BeginPlay event (issue UE-27284), I set "init settings" also in OnPostLogin event to be sure all settings was set right
  (Utilities|FlowControl|Sequence
    (:then_0
      (CallFunction|EInitSettings))
    (:then_1
      (NewPlayersProcessing|FSonPostLogin NewPlayer)
      (Utilities|FlowControl|Delay 0.5)
      (NewPlayersProcessing|FSDefineWhattoDowithPlayer NewPlayer))))

(event EventOnLogout
  (params (ExitingController :type Controller%20Object%20Reference))
  (bind _kernelgs (CallFunction|HKernelGS))
  ;[0 0.1238 1] LogOut event. Update session info
  (CallFunction|FSonLogout ExitingController)
  (Utilities|FlowControl|Delay 1.0)
  (if (and (<= (Default|FGetTotalPlayers _kernelgs) 1) (Utilities|Enum|Equal(Enum) (Variables|/Game/AMT/Blueprints/Kernel/BP_Kernel_GS.BP_Kernel_GS_C|GetGlobalState _kernelgs) "NewEnumerator17"))
    (Default|EAFinishPlayTime (CallFunction|HKernelGS))))

(fn ConstructionScript)

(fn FSonLogout
  (params (ExitingController :type Controller%20Object%20Reference))
  (bind _asplayer_controller (Utilities|Casting|CastToPlayerController ExitingController))
  (LocalVariables|SetExitingPCLocal _asplayer_controller)
  (Utilities|FlowControl|Sequence
    (:then_0
      (Class|BPIBasePlayerController|IEDisconnectfromtheServer(Message) (LocalVariables|GetExitingPCLocal)))
    (:then_1
      (Utilities|Array|RemoveItem (Variables|Players|GetConnectedPlayers) (LocalVariables|GetExitingPCLocal))
      (LocalVariables|SetExitingPCLocal 0))))

(fn FSonPostLogin
  (params (NewPC :type Player%20Controller%20Object%20Reference))
  (bind _output_get (LocalVariables|SetNewPC_L NewPC))
  (Utilities|FlowControl|Sequence
    (:then_0
      ;[1 1 1] disconnect new player if there is already maximim players on the server
      (if (Info|FSShouldDisconnectNewPlayer)
        (Class|BPIBasePlayerController|IEDisconnectfromtheServer(Message) (LocalVariables|GetNewPC_L))
        (return)))
    (:then_1
      (Utilities|Array|AddUnique (Variables|Players|GetConnectedPlayers) _output_get))))

(fn FSSpawnAllPlayers
  (for _array_element (Variables|Players|GetConnectedPlayers)
    (bind _asbp_kernel_ps (Utilities|Casting|CastToBP_Kernel_PS (Variables|/Script/Engine.Controller|GetPlayerState _array_element)))
    (PlayerRespawn|FSRespawnPlayer _array_element (PlayerRespawn|FSGetSpawnLocation (Default|FSIsCurrentMonster _asbp_kernel_ps) "0, 0, 0"))))

(fn FSDestroyAllPlayers
  (for _array_element (Variables|Players|GetConnectedPlayers)
    (Class|BPIBasePlayerController|IEDestroyControlledPawn(Message) _array_element)))

(fn FSRespawnPlayer
  (params (PC :type Player%20Controller%20Object%20Reference) (RespawnLocation :type Transform))
  (bind _output_get (LocalVariables|SetPC_L PC))
  (Class|BPIBasePlayerController|IEDestroyControlledPawn(Message) _output_get)
  (bind _returnvalue (Game|SpawnActorfromClass (PlayerRespawn|FSGetPawnClass _output_get) RespawnLocation "AdjustIfPossibleButAlwaysSpawn" (LocalVariables|GetPC_L) 0))
  (Utilities|IsValid _returnvalue
    (:Is%20Valid
      (Pawn|Possess (LocalVariables|GetPC_L) _returnvalue)
      (return _returnvalue))
    (:Is%20Not%20Valid
      (Development|PrintString "RESPAWN ERROR" true true "(R=1.000000,G=0.000000,B=0.000000,A=1.000000)" 22.0))))

(fn FSSetHostGameSettings
  (bind _maingi (CallFunction|HMainGI))
  (Variables|HostSettings|SetServerName (Variables|/Game/AMT/Blueprints/Kernel/BP_MainGI.BP_MainGI_C|GetServerName _maingi))
  (Variables|HostSettings|SetMinPlayersToStart (Variables|/Game/AMT/Blueprints/Kernel/BP_MainGI.BP_MainGI_C|GetMinPlayersToStart _maingi)))

(fn FSProcessPlayerDeath
  (params (VictimPS :type Player%20State%20Object%20Reference) (KillerPS :type Player%20State%20Object%20Reference))
  (LocalVariables|SetVictimPS_L VictimPS)
  (LocalVariables|SetKillerPS_L KillerPS)
  (Utilities|FlowControl|Sequence
    (:then_0
      ;[1 1 1] Update kills log
      (Default|MCUpdateKillFeed (CallFunction|HKernelGS) (Variables|/Script/Engine.PlayerState|GetPlayerId (LocalVariables|GetKillerPS_L)) (Variables|/Script/Engine.PlayerState|GetPlayerId (LocalVariables|GetVictimPS_L))))
    (:then_1
      ;[1 1 1] Show observer hud and spawn observer for victim
      (bind _asbp_kernel_ps (Utilities|Casting|CastToBP_Kernel_PS (LocalVariables|GetVictimPS_L)))
      (Default|EAonDeath _asbp_kernel_ps))
    (:then_2
      ;[1 1 1] Finish play time if the monster killed all players
      (if (<= (Default|FGetAlivePlayers (CallFunction|HKernelGS)) 0)
        (Default|EAFinishPlayTime (CallFunction|HKernelGS))))))

(fn FSSetGameModeSettingsforDedicatedServer
  (bind _returnvalue (Utilities|GetCommandLine))
  (LocalVariables|SetCommandLine _returnvalue)
  (Utilities|FlowControl|Sequence
    (:then_0
      ;[1 1 1] server name
      (Variables|HostSettings|SetServerName (CallFunction|HParseOption (LocalVariables|GetCommandLine) "sn")))
    (:then_1
      (Variables|HostSettings|SetMinPlayersToStart (Math|Conversions|ToInteger(Byte) (CallFunction|HParseOption (LocalVariables|GetCommandLine) "mn"))))))

(fn FCheckHostSettings
  (Utilities|FlowControl|Sequence
    (:then_0
      (Utilities|MHIsEmptyString (Variables|HostSettings|GetServerName)
        (:true
          (Variables|HostSettings|SetServerName "Unnamed Server"))))
    (:then_1
      (if (<= (Variables|HostSettings|GetMinPlayersToStart) 1)
        (Variables|HostSettings|SetMinPlayersToStart 2)))))

(fn FSShouldDisconnectNewPlayer
  (return (>= (Default|FGetTotalPlayers (CallFunction|HKernelGS)) (Variables|HostSettings|GetMaxPlayers))))

(fn FSGetSpawnLocation
  (params (IsMonster :type Boolean) (Location :type Vector))
  (bind _playersspawnpoints_l (LocalVariables|GetPlayersSpawnPoints_L))
  (bind _monsterspawnpoints_l (LocalVariables|GetMonsterSpawnPoints_L))
  (bind _returnvalue (Utilities|Array|Length _playersspawnpoints_l))
  (bind _output (Utilities|Array|Get(acopy) _monsterspawnpoints_l))
  (bind _returnvalue_2 (- _returnvalue 1))
  (bind _returnvalue_3 (Math|Random|RandomInteger _returnvalue_2))
  (bind _output_2 (Utilities|Array|Get(acopy) _playersspawnpoints_l _returnvalue_3))
  (Utilities|FlowControl|Sequence
    (:then_0
      (bind _outactors (Actor|GetAllActorsOfClass "/Game/AMT/Blueprints/Kernel/BP_SpawnPoint.BP_SpawnPoint_C"))
      (for _array_element _outactors
        (if (Variables|/Game/AMT/Blueprints/Kernel/BP_SpawnPoint.BP_SpawnPoint_C|GetIsMonster _array_element)
          (Utilities|Array|AddUnique (LocalVariables|GetMonsterSpawnPoints_L) _array_element)
          (else
            (Utilities|Array|AddUnique (LocalVariables|GetPlayersSpawnPoints_L) _array_element)))))
    (:then_1
      (if IsMonster
        (Utilities|IsValid _output
          (:Is%20Valid
            (return (Transformation|GetActorTransform _output)))
          (:Is%20Not%20Valid
            (return (Math|Transform|MakeTransform "0, 0,300.000000"))))
        (else
          (Utilities|IsValid _output_2
            (:Is%20Valid
              (return (Transformation|GetActorTransform _output_2)))
            (:Is%20Not%20Valid
              (return (Math|Transform|MakeTransform "0, 0,300.000000")))))))))

(fn FSGetPawnClass
  (params (PC :type Player%20Controller%20Object%20Reference))
  (bind _asbp_kernel_ps (Utilities|Casting|CastToBP_Kernel_PS (Variables|/Script/Engine.Controller|GetPlayerState PC)))
  (if (Default|FSIsCurrentMonster _asbp_kernel_ps)
    (return "/Game/AMT/Blueprints/Characters/BP_Monster.BP_Monster_C")
    (else
      (return "/Game/AMT/Blueprints/Characters/BP_Player.BP_Player_C"))))

(fn FSDefineWhattoDowithPlayer
  (params (PC :type Player%20Controller%20Object%20Reference))
  (LocalVariables|SetPC_L PC)
  (switch Utilities|FlowControl|Switch|SwitchonE_GlobalState (Variables|/Game/AMT/Blueprints/Kernel/BP_Kernel_GS.BP_Kernel_GS_C|GetGlobalState (CallFunction|HKernelGS))
    (:NewEnumerator28
      (PlayerRespawn|FSRespawnPlayer (LocalVariables|GetPC_L) (PlayerRespawn|FSGetSpawnLocation false "0, 0, 0")))
    (:NewEnumerator17
      (bind _asbp_kernel_ps (Utilities|Casting|CastToBP_Kernel_PS (Variables|/Script/Engine.Controller|GetPlayerState (LocalVariables|GetPC_L))))
      (Default|FSSpawnObserverPawn _asbp_kernel_ps))))

(fn FSMakeRandomPlayerMonster
  (bind _array_element (Utilities|Array|ForEachLoopwithBreak (Variables|Players|GetConnectedPlayers) :!label _label)
    (:LoopBody
      (bind _asbp_kernel_ps (Utilities|Casting|CastToBP_Kernel_PS (Variables|/Script/Engine.Controller|GetPlayerState _array_element)))
      (if (Default|FSCanbeMonster _asbp_kernel_ps)
        (Variables|/Game/AMT/Blueprints/Kernel/BP_Kernel_PS.BP_Kernel_PS_C|SetIsMonster _asbp_kernel_ps true)
        (LocalVariables|SetMonsterWasSet_L true)
        (goto _label Break)))
    (:Completed
      (if (LocalVariables|GetMonsterWasSet_L)
        (return)
        (else
          (Monster|FSClearMonsterStateforAll)
          (Monster|FSMakeRandomPlayerMonster))))))

(fn FSClearMonsterStateforAll
  (for _array_element (Variables|Players|GetConnectedPlayers)
    (bind _asbp_kernel_ps (Utilities|Casting|CastToBP_Kernel_PS (Variables|/Script/Engine.Controller|GetPlayerState _array_element)))
    (Variables|/Game/AMT/Blueprints/Kernel/BP_Kernel_PS.BP_Kernel_PS_C|SetIsMonster _asbp_kernel_ps false)
    (Variables|/Game/AMT/Blueprints/Kernel/BP_Kernel_PS.BP_Kernel_PS_C|SetPlayedAsMonster _asbp_kernel_ps false)))